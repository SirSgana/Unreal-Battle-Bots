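; BP_SmallSphere is a short-lived moving pickup that scores a point when a DefaultPawn overlaps it.
; BeginPlay scales it in, picks a random spin and starts a lifetime timer.
; Tick moves it along its rotating forward vector without sweep, giving it a turning path.
; Overlap increments BP_BadBotGameMode's score; overlap or timeout triggers a guarded scale timeline that destroys the actor when finished.
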(event `self.ReceiveTick`
  (params (DeltaSeconds :type "Float (single-precision)"))
  ;[0 0.816 0.8073 0.5] Movimento e Rotazione Sfera
  (`self.K2_AddActorWorldOffset` (* (`self.GetActorForwardVector`) (* DeltaSeconds (`self.Speed`))))
  (`self.K2_AddActorWorldRotation` (* (`self.Delta Rotation`) DeltaSeconds)))

(event `self.ReceiveBeginPlay`
  (`self.WinkIn`)
  (set `self.Delta Rotation` (* (`KismetMathLibrary.RandomRotator` false) (`self.RotationScaleFactor`)))
  ;[0.7887 0.1272 0.6769 0.5] Start Wink Out
  (`KismetSystemLibrary.K2_SetTimerDelegate` (delegate `WinkOut`) (`self.LifeTime`))
  ;[0.6615 0.1719 0.1404 0.5] Event Begin Overlap and Score Up
  (add `PrimitiveComponent.OnComponentBeginOverlap` (`self.SphereVolume`) (delegate `On Sphere Overlap`)))

(event `On Sphere Overlap`
  (params (OverlappedComponent :type "PrimitiveComponent Object Reference") (OtherActor :type "Actor Object Reference") (OtherComp :type "PrimitiveComponent Object Reference") (OtherBodyIndex :type Integer) (bFromSweep :type Boolean) (SweepResult :type "HitResult Structure (by ref)"))
  ;[0.6615 0.1719 0.1404 0.5] Event Begin Overlap and Score Up
  (if (`GameplayStatics.ObjectIsA` OtherActor "/Script/Engine.DefaultPawn")
    (bind _asbp_bad_bot_game_mode (cast `/Game/BluePrints/Game/BP_BadBotGameMode` (`GameplayStatics.GetGameMode`)))
    (`/Game/BluePrints/Game/BP_BadBotGameMode.Increment Score` _asbp_bad_bot_game_mode)
    (`self.WinkOut`)))

(event `WinkOut`
  ;[0.7887 0.1272 0.6769 0.5] Start Wink Out
  (if (not (`self.IsWinking`))
    (set `self.IsWinking` true)
    (bind (_direction _scale) (`Timeline|WinkOutTimeline`)
      (:`Update`
        (`SceneComponent.SetWorldScale3D` (`self.SmallSphere`) (`KismetMathLibrary.MakeVector` _scale _scale _scale)))
      (:`Finished`
        (`self.K2_DestroyActor`)))))

(event `WinkIn`
  ;[0.7796 0.1925 0.6618 0.5] Wink In to Existent
  (bind (_direction _scale) (`Timeline|WinkInTimeline`)
    (:`Update`
      (`SceneComponent.SetWorldScale3D` (`self.SmallSphere`) _scale))))

(fn `UserConstructionScript`)